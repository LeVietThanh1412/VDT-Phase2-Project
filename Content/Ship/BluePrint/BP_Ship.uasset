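; Player-controlled, physics-driven warship with buoyancy, Enhanced Input movement and an aimable front gun.
; Forward thrust and speed-scaled turning forces at hull sockets apply only in water; an interpolated ForceFactor tracks throttle.
; Aiming switches to a zoomable gun camera and line-traces from the muzzle each tick to drive the crosshair.
; Firing spawns projectiles, using a suggested toss velocity on hits, plus effects and a recoil timeline that gates refire.
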(event Custom|EngineManager
  (if (> (Input|EnhancedActionValues|GetIA_MoveForwardBackward) 0.0)
    (Variables|Default|SetForceFactor (Math|Interpolation|FInterpTo (Variables|Default|GetForceFactor) 1.0 (Utilities|Time|GetWorldDeltaSeconds) 2e+01))
    (elif (== (Input|EnhancedActionValues|GetIA_MoveForwardBackward) 0.0)
      (Variables|Default|SetForceFactor (Math|Interpolation|FInterpTo (Variables|Default|GetForceFactor) 0.0 (Utilities|Time|GetWorldDeltaSeconds) 2.0))
      (else
        (Variables|Default|SetForceFactor (Math|Interpolation|FInterpTo (Variables|Default|GetForceFactor) -1.0 (Utilities|Time|GetWorldDeltaSeconds) 2.0))))))

(event Custom|ManageAiming
  (bind _ship (Variables|Default|GetShip))
  (bind _returnvalue (Transformation|GetSocketLocation _ship "front_gun_v_socket"))
  (if (Components|Activation|IsActive (Variables|Default|GetGunCamera))
    (bind _outhit (Collision|LineTraceByChannel _returnvalue (+ _returnvalue (* (Math|Vector|GetForwardVector (Transformation|GetSocketRotation _ship "front_gun_v_socket")) 99999999.0)) "TraceTypeQuery1" false 0 "ForOneFrame" false))
    (bind _output_get (Variables|Default|SetIs%20Hit (.bBlockingHit (Collision|BreakHitResult _outhit))))
    (if _output_get
      (if (== (.HitActor (Collision|BreakHitResult _outhit)) self)
        (Rendering|SetVisibility (Variables|Default|GetCrosshair) false false)
        (else
          (Variables|Default|SetImpact%20Point (.ImpactNormal (Collision|BreakHitResult _outhit)))
          (Transformation|SetWorldLocation (Variables|Default|GetCrosshair) (Variables|Default|GetImpact%20Point) false false :!label _label)
          (Rendering|SetVisibility (Variables|Default|GetCrosshair) true false)))
      (else
        (Variables|Default|SetImpact%20Point (.TraceEnd (Collision|BreakHitResult _outhit)))
        (goto _label)))))

(event Input|EnhancedActionEvents|EnhancedInputActionIA_LookAround
  (params (ActionValue :type Vector%202D%20Structure) (ElapsedSeconds :type Float%20%28double-precision%29) (TriggeredSeconds :type Float%20%28double-precision%29) (InputAction :type Input%20Action%20Object%20Reference :default "/Game/Ship/Inputs/IA_LookAround.IA_LookAround"))
  (bind (_x _y) (Math|Vector2D|BreakVector2D ActionValue))
  (Pawn|Input|AddControllerYawInput _x)
  (Pawn|Input|AddControllerPitchInput _y))

(event Input|EnhancedActionEvents|EnhancedInputActionIA_MoveForwardBackward
  (params (ActionValue :type Float%20%28double-precision%29) (ElapsedSeconds :type Float%20%28double-precision%29) (TriggeredSeconds :type Float%20%28double-precision%29) (InputAction :type Input%20Action%20Object%20Reference :default "/Game/Ship/Inputs/IA_MoveForwardBackward.IA_MoveForwardBackward"))
  (if (Buoyancy|IsinWaterBody (Variables|Default|GetBuoyancy))
    (Physics|AddForce (Variables|Default|GetShipSM) (* (* (Math|Vector|GetForwardVector (Variables|Default|GetArrow)) 3.2e+05) ActionValue) "None" false)))

(event Input|EnhancedActionEvents|EnhancedInputActionIA_Aim
  (params (ActionValue :type Boolean) (ElapsedSeconds :type Float%20%28double-precision%29) (TriggeredSeconds :type Float%20%28double-precision%29) (InputAction :type Input%20Action%20Object%20Reference :default "/Game/Ship/Inputs/IA_Aim.IA_Aim"))
  (bind _crosshair (Variables|Default|GetCrosshair))
  (:Started
    (Components|Activation|SetActive (Variables|Default|GetGunCamera) true false)
    (Components|Activation|SetActive (Variables|Default|GetCamera) false false)
    (Rendering|SetVisibility _crosshair true false))
  (:Completed
    (Components|Activation|SetActive (Variables|Default|GetGunCamera) false false)
    (Components|Activation|SetActive (Variables|Default|GetCamera) true false)
    (Rendering|SetVisibility _crosshair false false)
    (Camera|SetFieldOfView (Variables|Default|GetGunCamera) 9e+01)))

(event Input|EnhancedActionEvents|EnhancedInputActionIA_MoveLeftRight
  (params (ActionValue :type Float%20%28double-precision%29) (ElapsedSeconds :type Float%20%28double-precision%29) (TriggeredSeconds :type Float%20%28double-precision%29) (InputAction :type Input%20Action%20Object%20Reference :default "/Game/Ship/Inputs/IA_MoveLeftRight.IA_MoveLeftRight"))
  (bind _shipsm (Variables|Default|GetShipSM))
  (bind _shipsm_2 (Variables|Default|GetShipSM))
  (bind _shipsm_3 (Variables|Default|GetShipSM))
  (bind _shipsm_4 (Variables|Default|GetShipSM))
  (if (and (Buoyancy|IsinWaterBody (Variables|Default|GetBuoyancy)) (> (CallFunction|GetSpeed) 5.0))
    (if (> (Math|Float|Sign(Float) ActionValue) 0.0)
      (Class|PrimitiveComponent|AddForceatLocationLocal (Variables|Default|GetShipSM) (* (Math|Vector|GetRightVector (Math|Transform|InverseTransformRotation (Transformation|GetWorldTransform _shipsm_2) (Transformation|GetSocketRotation _shipsm_2 "5"))) (Math|Float|MapRangeClamped (CallFunction|GetSpeed) 0.0 2e+01 5e+03 1.6e+04)) (Math|Transform|InverseTransformLocation (Transformation|GetWorldTransform _shipsm_3) (Transformation|GetSocketLocation _shipsm_3 "5")) "None")
      (else
        (Class|PrimitiveComponent|AddForceatLocationLocal (Variables|Default|GetShipSM) (* (Math|Vector|NegateVector (Math|Vector|GetRightVector (Math|Transform|InverseTransformRotation (Transformation|GetWorldTransform _shipsm) (Transformation|GetSocketRotation _shipsm "4")))) (Math|Float|MapRangeClamped (CallFunction|GetSpeed) 0.0 2e+01 5e+03 1.6e+04)) (Math|Transform|InverseTransformLocation (Transformation|GetWorldTransform _shipsm_4) (Transformation|GetSocketLocation _shipsm_4 "4")) "None")))))

(event Input|EnhancedActionEvents|EnhancedInputActionIA_Fire
  (params (ActionValue :type Boolean) (ElapsedSeconds :type Float%20%28double-precision%29) (TriggeredSeconds :type Float%20%28double-precision%29) (InputAction :type Input%20Action%20Object%20Reference :default "/Game/Ship/Inputs/IA_Fire.IA_Fire"))
  (:Started
    (if (Math|Boolean|ANDBoolean (Rendering|IsVisible (Variables|Default|GetCrosshair)) (Components|Activation|IsActive (Variables|Default|GetGunCamera)) (Variables|Default|GetCanShoot))
      (if (Variables|Default|GetIs%20Hit)
        (bind _tossvelocity (Class|GameplayStatics|BlueprintSuggestProjectileVelocity (Transformation|GetSocketLocation (Variables|Default|GetShip) "front_gun_v_socket") (Variables|Default|GetImpact%20Point) 2e+04 0.0 "DoNotTrace" 0.0 false false false))
        (Game|SpawnActorfromClass "/Game/Ship/BluePrint/BP_ShipProjectileWithSpeed.BP_ShipProjectileWithSpeed_C" (Transformation|GetSocketTransform (Variables|Default|GetShip) "front_gun_v_socket" "RTS_World") "Undefined" "MultiplyWithRoot" 0 _tossvelocity 0)
        (else
          (Game|SpawnActorfromClass "/Game/Ship/BluePrint/BP_ShipProjectile.BP_ShipProjectile_C" (Transformation|GetSocketTransform (Variables|Default|GetShip) "front_gun_v_socket" "RTS_World") "Undefined" "MultiplyWithRoot" 0 0)))
      (Niagara|SpawnSystemAttached "/Game/Ship/Assets/VigilanteContent/Vehicles/West_Ship_DDG102/FX/NS_West_Ship_DDG102_FrontGuns.NS_West_Ship_DDG102_FrontGuns" (Variables|Default|GetShip) "front_gun_v_socket" "0, 0, 0" "0, 0, 0" "KeepRelativeOffset" false)
      (Audio|SpawnSoundatLocation "/Game/Ship/Assets/Audio/ES_Cannon_Fire_1_-_SFX_Producer.ES_Cannon_Fire_1_-_SFX_Producer" (Transformation|GetSocketLocation (Variables|Default|GetShip) "None") "0, 0, 0" 1.0 1.0 0.0 0 0)
      (bind _recoilvalue (Timeline|Recoil PlayFromStart)
        (:Update
          (Variables|Default|SetRecoil%20Value _recoilvalue)
          (Variables|Default|SetCanShoot false))
        (:Finished
          (Variables|Default|SetCanShoot true))))))

(event Input|EnhancedActionEvents|EnhancedInputActionIA_Zoom
  (params (ActionValue :type Float%20%28double-precision%29) (ElapsedSeconds :type Float%20%28double-precision%29) (TriggeredSeconds :type Float%20%28double-precision%29) (InputAction :type Input%20Action%20Object%20Reference :default "/Game/Ship/Inputs/IA_Zoom.IA_Zoom"))
  (Camera|SetFieldOfView (Variables|Default|GetGunCamera) (Math|Float|Clamp(Float) (+ (Variables|/Script/Engine.CameraComponent|GetFieldOfView (Variables|Default|GetGunCamera)) (* ActionValue 5.0)) 6e+01 1.2e+02)))

(event EventBeginPlay
  (Input|AddMappingContext (PlayerController|LocalPlayerSubsystems|GetEnhancedInputLocalPlayerSubsystem (Game|GetPlayerController 0)) "/Game/Ship/Inputs/IMC_Ship.IMC_Ship" 0 "(bIgnoreAllPressedKeysUntilRelease=True,bForceImmediately=False,bNotifyUserSettings=False)")
  (Components|Activation|SetActive (Variables|Default|GetGunCamera) false false)
  (Components|Activation|SetActive (Variables|Default|GetCamera) true false))

(event Collision|EventActorBeginOverlap
  (params (OtherActor :type Actor%20Object%20Reference)))

(event EventTick
  (params (DeltaSeconds :type Float%20%28single-precision%29))
  (CallFunction|EngineManager)
  (CallFunction|ManageAiming))

(fn ConstructionScript)

(fn GetSpeed
  (return (/ (Math|Vector|VectorLengthXY (Transformation|GetVelocity)) 1e+02)))