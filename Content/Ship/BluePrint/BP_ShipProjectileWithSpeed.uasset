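; Ship projectile Blueprint that flies at a supplied velocity and explodes where it stops.
; On BeginPlay, it copies its Speed variable into the ProjectileMovement velocity.
; When the movement stops, it applies heavy radial damage at the impact point, spawns a normal-aligned Niagara explosion and positional sound, then destroys itself.
; A debug sphere showing the damage radius is also drawn on impact.
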(event OnProjectileStop(ProjectileMovement)
  (params (ImpactResult :type Hit%20Result%20Structure%20%28by%20ref%29))
  (bind (_bblockinghit _binitialoverlap _time _distance _location _impactpoint _normal _impactnormal) (Collision|BreakHitResult ImpactResult))
  (bind _self self)
  (Game|Damage|ApplyRadialDamage 1e+04 _impactpoint 1e+03 0 (Utilities|Array|MakeArray _self) _self 0 false "ECC_Visibility")
  (Rendering|Debug|DrawDebugSphere _impactpoint 1e+03 12 "(R=1.000000,G=0.000000,B=0.000000,A=1.000000)" 5.0 1e+01)
  (Niagara|SpawnSystematLocation "/Game/Ship/Assets/MsvFx_Niagara_Explosion_Pack_01/Prefabs/Niagara_Dust_Explosion_01.Niagara_Dust_Explosion_01" _impactpoint (Math|Rotator|MakeRotfromX _impactnormal))
  (Audio|SpawnSoundatLocation "/Game/Ship/Assets/Audio/ES_Grenade_Explosion_14_-_SFX_Producer.ES_Grenade_Explosion_14_-_SFX_Producer" _impactpoint "0, 0, 0" 1.0 1.0 0.0 "/Game/Ship/Sound/NewSoundAttenuation.NewSoundAttenuation" 0)
  (Actor|DestroyActor))

(event EventBeginPlay
  (Variables|/Script/Engine.MovementComponent|SetVelocity (Variables|Default|GetProjectileMovement) (Variables|Default|GetSpeed)))

(event Collision|EventActorBeginOverlap
  (params (OtherActor :type Actor%20Object%20Reference)))

(event EventTick
  (params (DeltaSeconds :type Float%20%28single-precision%29)))

(fn ConstructionScript)