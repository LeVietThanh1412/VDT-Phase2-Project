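; BP_AntiShip is an anti-ship gun that targets the player's BP_Ship and fires projectiles at it.
; Each tick, a box trace from the gun socket sets CanShoot when it hits the ship, and a look-at rotation updates GunPitch.
; A looping timer checks CanShoot, then spawns the projectile with muzzle flash, shell ejection and sound, while a timeline drives RecoilValue.
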(event Custom|LightofSightManager
  (bind _skeletalmesh (Variables|Default|GetSkeletalMesh))
  (bind _returnvalue (Transformation|GetSocketLocation _skeletalmesh "gun_jntSocket"))
  (bind _outhit (Collision|BoxTraceByChannel _returnvalue (+ _returnvalue (* (Math|Vector|GetForwardVector (Transformation|GetSocketRotation _skeletalmesh "gun_jntSocket")) 1e+05)) "10.000000,10.000000,100.000000" "0, 0, 0" "TraceTypeQuery1" false 0 "ForOneFrame"))
  (if (.bBlockingHit (Collision|BreakHitResult _outhit))
    (if (== (.HitActor (Collision|BreakHitResult _outhit)) (Variables|Default|GetTarget))
      (Variables|Default|SetCanShoot true)
      (else
        (Variables|Default|SetCanShoot false)))
    (else
      (Variables|Default|SetCanShoot false))))

(event Custom|GunDirectionManager
  (Utilities|IsValid (Variables|Default|GetTarget)
    (:Is%20Valid
      (Variables|Default|SetGunPitch (.pitch (Math|Rotator|Delta(Rotator) (Math|Rotator|FindLookatRotation (Transformation|GetActorLocation) (Transformation|GetActorLocation (Variables|Default|GetTarget))) (Transformation|GetActorRotation)))))))

(event Custom|Fire
  (if (Variables|Default|GetCanShoot)
    (Game|SpawnActorfromClass "/Game/AntiShip/BluePrint/BP_AntiShipProjectile.BP_AntiShipProjectile_C" (Transformation|GetSocketTransform (Variables|Default|GetSkeletalMesh) "gun_jntSocket" "RTS_World") "Undefined" "MultiplyWithRoot" 0 0)
    (Components|Activation|SetActive (Variables|Default|GetMuzzleFlash) true true)
    (Audio|SpawnSoundatLocation "/Game/Ship/Assets/Audio/ES_Cannon_Fire_1_-_SFX_Producer.ES_Cannon_Fire_1_-_SFX_Producer" (Transformation|GetActorLocation) "0, 0, 0" 1.0 1.0 0.0 "/Game/Ship/Sound/NewSoundAttenuation.NewSoundAttenuation" 0)
    (bind _recoilvalue (Timeline|Recoil PlayFromStart)
      (:Update
        (Variables|Default|SetRecoil%20Value _recoilvalue)))))

(event EventBeginPlay
  (bind _asbp_ship (Utilities|Casting|CastToBP_Ship (Game|Player|GetPlayerPawn 0)))
  (Variables|Default|SetTarget _asbp_ship)
  (Utilities|Time|SetTimerbyEvent (delegate Custom|Fire) 5.0 true))

(event Collision|EventActorBeginOverlap
  (params (OtherActor :type Actor%20Object%20Reference)))

(event EventTick
  (params (DeltaSeconds :type Float%20%28single-precision%29))
  (CallFunction|LightofSightManager)
  (CallFunction|GunDirectionManager))

(fn ConstructionScript)